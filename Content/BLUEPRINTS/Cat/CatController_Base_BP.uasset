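; Base AI controller for the cat that makes it wander endlessly around the navmesh.
; On BeginPlay it moves the pawn to a random navigable point within a radius of its current location.
; Tick polls the path-following status and, when it changes to Idle, fires MoveFinished, which picks the next roam point.
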(event Custom|Roam
  (CallFunction|Roaming))

(event Custom|MoveFinished
  (CallFunction|Roam))

(event EventTick
  (params (DeltaSeconds :type Float%20%28single-precision%29))
  (CallFunction|UpdateMove))

(event EventBeginPlay
  (CallFunction|Roam))

(fn ConstructionScript)

(fn Roaming
  (bind _randomlocation (Class|NavigationSystemV1|GetRandomLocationinNavigableRadius (Transformation|GetActorLocation (Pawn|GetControlledPawn)) 1e+03 0 0))
  (AI|Navigation|MovetoLocation _randomlocation 2e+01 false true false false 0))

(fn UpdateMove
  (bind _returnvalue (Class|AIController|GetMoveStatus))
  (Utilities|FlowControl|Sequence
    (:then_0
      (if (and (!= (Variables|Default|GetMoveStatus) _returnvalue) (Utilities|Enum|Equal(Enum) _returnvalue "Idle"))
        (CallFunction|MoveFinished)))
    (:then_1
      (Variables|Default|SetMoveStatus _returnvalue))))